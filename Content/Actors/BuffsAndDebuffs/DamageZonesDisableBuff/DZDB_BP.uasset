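; DZDB_BP is a pickup buff that temporarily disables damage zones (static traps) by clearing IsDamageZonesOn on the DDO_PlayerState.
; On BeginPlay it reads Duration from a settings DataTable row chosen by the GameState's hard or easy room flag, then spins via a timeline.
; On overlap it clears the flag, teleports itself to a fixed location instead of being destroyed, and a timer restores the flag after Duration.
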(event `self.ReceiveActorBeginOverlap`
  (params (OtherActor :type "Actor Object Reference"))
  ;[0.2122 0.2122 0.2122 0.498] Отключение статических ловушек на время Duration
  (bind _asddo_player_state (cast `/Game/GameplayFramework/DDO_PlayerState` (`GameplayStatics.GetPlayerState` 0)))
  (set `/Game/GameplayFramework/DDO_PlayerState.IsDamageZonesOn` false _asddo_player_state)
  (`KismetSystemLibrary.K2_SetTimerDelegate` (delegate `Stop`) (`self.Duration`))
  (`self.K2_TeleportTo` (-1800.0 0.0 0.0)))

(event `Stop`
  ;[0.2122 0.2122 0.2122 0.498] Отключение статических ловушек на время Duration
  (set `/Game/GameplayFramework/DDO_PlayerState.IsDamageZonesOn` true (stale `self.ReceiveActorBeginOverlap` _asddo_player_state)))

(event `self.ReceiveBeginPlay`
  ;[0.2122 0.2122 0.2122 0.498] Инициализация и последующее вращение объекта
  (`self.SetupDZDB`)
  (bind (_direction _rotation) (`Timeline|Rotation_TL`)
    (:`Update`
      (`SceneComponent.K2_AddRelativeRotation` (`self.DefaultSceneRoot`) (`KismetMathLibrary.MakeRotator` 0.0 0.0 _rotation) false false))))

(fn `SetupDZDB`
  ;[0.2122 0.2122 0.2122 0.498] Вычитывание настроек из таблицы
  (bind _asddo_game_state (cast `/Game/GameplayFramework/DDO_GameState` (`GameplayStatics.GetGameState`)))
  (if (`/Game/GameplayFramework/DDO_GameState.IsCurrentRoomHard` _asddo_game_state)
    (bind _returnvalue (`|GetDataTableRow` "/Game/Actors/BuffsAndDebuffs/DamageZonesDisableBuff/DZDBSettings_Table.DZDBSettings_Table" "HardRoom")
      (:`then`
        (set `self.Duration` (break `/Game/Actors/BuffsAndDebuffs/DamageZonesDisableBuff/DZDBSettings_Struct` _returnvalue))))
    (else
      (bind _returnvalue_2 (`|GetDataTableRow` "/Game/Actors/BuffsAndDebuffs/DamageZonesDisableBuff/DZDBSettings_Table.DZDBSettings_Table" "EasyRoom")
        (:`then`
          (set `self.Duration` (break `/Game/Actors/BuffsAndDebuffs/DamageZonesDisableBuff/DZDBSettings_Struct` _returnvalue_2)))))))

(fn `UserConstructionScript`)