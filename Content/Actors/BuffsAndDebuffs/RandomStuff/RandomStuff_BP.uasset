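; RandomStuff_BP is a rotating mystery pickup that turns into a random buff or debuff when overlapped, intended for the player.
; On overlap it randomly spawns MTSB_BP, DZDB_BP or PlayerSlowingDebuff_BP, teleports it to its own location and destroys itself.
; The overlap event does not check which actor touched it.
; A timeline started on BeginPlay adds yaw to the root component to spin it.
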(event `self.ReceiveActorBeginOverlap`
  (params (OtherActor :type "Actor Object Reference"))
  (bind _returnvalue (`self.K2_GetActorLocation` self))
  ;[0.2122 0.2122 0.2122 0.498] Спавн рандомного бафа/дебава при столкновении с игроком
  (switch `int` (`KismetMathLibrary.RandomIntegerInRange` 0 2)
    (:`Default`
      (bind _returnvalue_2 (`|SpawnActorFromClass` "/Game/Actors/BuffsAndDebuffs/PlayerSlowingDebuff/PlayerSlowingDebuff_BP.PlayerSlowingDebuff_BP_C" (`KismetMathLibrary.MakeTransform` (0.0 0.0 0.0)) "AlwaysSpawn" "OverrideRootScale" null null))
      (`self.K2_TeleportTo` :`self` _returnvalue_2 :`DestLocation` _returnvalue))
    (:`0`
      (bind _returnvalue_3 (`|SpawnActorFromClass` "/Game/Actors/BuffsAndDebuffs/MovingTrapSlowingBuff/MTSB_BP.MTSB_BP_C" (`KismetMathLibrary.MakeTransform` (0.0 0.0 0.0)) "Undefined" "OverrideRootScale" null null))
      (`self.K2_TeleportTo` :`self` _returnvalue_3 :`DestLocation` _returnvalue))
    (:`1`
      (bind _returnvalue_4 (`|SpawnActorFromClass` "/Game/Actors/BuffsAndDebuffs/DamageZonesDisableBuff/DZDB_BP.DZDB_BP_C" (`KismetMathLibrary.MakeTransform` (0.0 0.0 0.0)) "Undefined" "OverrideRootScale" null null))
      (`self.K2_TeleportTo` :`self` _returnvalue_4 :`DestLocation` _returnvalue)))
  (`self.K2_DestroyActor`))

(event `self.ReceiveBeginPlay`
  ;[0.2122 0.2122 0.2122 0.498] Инициализация и последующее вращение объекта
  (bind (_direction _rotation) (`Timeline|Rotation_TL`)
    (:`Update`
      (`SceneComponent.K2_AddRelativeRotation` (`self.DefaultSceneRoot`) (`KismetMathLibrary.MakeRotator` 0.0 0.0 _rotation) false false))))

(fn `UserConstructionScript`)