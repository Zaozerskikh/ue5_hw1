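; Final stone pickup actor that serves as the win objective of the game.
; On BeginPlay it teleports itself to a random spot within a fixed area at constant height, then plays a timeline that spins its root around yaw.
; Any actor overlap, meant for the player but not filtered, sets IsStoneCollected on DDO_GameMode to signal the win.
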(event `self.ReceiveActorBeginOverlap`
  (params (OtherActor :type "Actor Object Reference"))
  ;[0.2122 0.2122 0.2122 0.498] Обработка столкновения с игроком (конец игры с выигрышем)
  (bind _asddo_game_mode (cast `/Game/GameplayFramework/DDO_GameMode` (`GameplayStatics.GetGameMode`)))
  (set `/Game/GameplayFramework/DDO_GameMode.IsStoneCollected` true _asddo_game_mode))

(event `self.ReceiveBeginPlay`
  ;[0.2122 0.2122 0.2122 0.498] Инициализация камня и его вращение
  (`self.SetupFinalStone`)
  (bind (_direction _rotation) (`Timeline|Rotation_TL`)
    (:`Update`
      (`SceneComponent.K2_AddRelativeRotation` (`self.DefaultSceneRoot`) (`KismetMathLibrary.MakeRotator` 0.0 0.0 _rotation) false false))))

(fn `SetupFinalStone`
  ;[0.2122 0.2122 0.2122 0.498] Спавн камня в рандомном месте
  (`self.K2_TeleportTo` (`KismetMathLibrary.MakeVector` (`KismetMathLibrary.RandomFloatInRange` 11000.0 11200.0) (`KismetMathLibrary.RandomFloatInRange` 800.0 2400.0) 50.0)))

(fn `UserConstructionScript`)