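; Room door actor that swings open while an actor overlaps it and signals a room change through its frame.
; The Door timeline drives the yaw of SMDoor, playing on begin overlap and reversing on end overlap.
; An overlap on SM_DoorFrame calls the teleport dispatcher with the door itself, then blocks further calls with a flag that a five-second timer resets.
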(event `self.ReceiveActorBeginOverlap`
  (params (OtherActor :type "Actor Object Reference"))
  ;[0.2122 0.2122 0.2122] Открывание/Закрывание двери
  (bind (_direction _open_close) (`Timeline|Door` :!label _label)
    (:`Update`
      (`SceneComponent.K2_SetRelativeRotation` (`self.SM_Door`) (`KismetMathLibrary.MakeRotator` 0.0 0.0 _open_close) false false))))

(event `self.ReceiveActorEndOverlap`
  (params (OtherActor :type "Actor Object Reference"))
  ;[0.2122 0.2122 0.2122] Открывание/Закрывание двери
  (goto _label :!via `Reverse`))

(event `self.SM_DoorFrame.OnComponentBeginOverlap`
  (params (OverlappedComponent :type "PrimitiveComponent Object Reference") (OtherActor :type "Actor Object Reference") (OtherComp :type "PrimitiveComponent Object Reference") (OtherBodyIndex :type Integer) (bFromSweep :type Boolean) (SweepResult :type "HitResult Structure (by ref)"))
  ;[0.2122 0.2122 0.2122] Смена комнаты
  (if (`self.IsUserNotTeleported`)
    (set `self.IsUserNotTeleported` false)
    (`self.TeleportDispatcher` self)
    (`KismetSystemLibrary.K2_SetTimerDelegate` (delegate `ResetTeleported`) 5.0)))

(event `ResetTeleported`
  ;[0.2122 0.2122 0.2122] Смена комнаты
  (set `self.IsUserNotTeleported` true))

(fn `UserConstructionScript`)