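; Moving oak trap that crosses the room along X and damages the player on overlap.
; On BeginPlay it randomizes its scale and height, teleports to the far end aligned with the player's Y, and reads damage and speed from DDO_GameState.
; A Timeline drives movement, scaled by an externally settable slowing factor, until the trap passes the opposite boundary.
; Any overlap reduces player health through DDO_PlayerState and destroys the trap.
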(event `self.ReceiveActorBeginOverlap`
  (params (OtherActor :type "Actor Object Reference"))
  ;[0.2122 0.2122 0.2122] Столкновение с игроком
  (bind _asddo_player_state (cast `/Game/GameplayFramework/DDO_PlayerState` (`GameplayStatics.GetPlayerState` 0)))
  (`/Game/GameplayFramework/DDO_PlayerState.ChangeHealth` _asddo_player_state (* (`self.Damage`) -1.0) "NewEnumerator0")
  (`self.K2_DestroyActor`))

(event `self.ReceiveBeginPlay`
  (bind (_returnvalue_x _returnvalue_y _returnvalue_z) (`KismetMathLibrary.BreakVector` (`self.K2_GetActorLocation` self)))
  ;[0.2122 0.2122 0.2122] Движение и самоуничтожение при достижении противоположной границы комнаты
  (`self.SetupOakTrap`)
  (bind (_direction _move) (`Timeline|Timeline`)
    (:`Update`
      (bind _returnvalue (+ _returnvalue_x (* _move (* (`self.Speed`) (`self.SlowingFactor`)))))
      (`self.K2_SetActorLocation` (`KismetMathLibrary.MakeVector` _returnvalue _returnvalue_y _returnvalue_z))
      (if (`self.IsAlive`)
        (if (< _returnvalue 200.0)
          (`self.K2_DestroyActor`))))))

(event `/Game/Actors/Traps/MovingTraps/IMovable.Set Slowing Factor`
  (params (SlowingFactor :type "Float (double-precision)"))
  ;[0.2122 0.2122 0.2122] Движение и самоуничтожение при достижении противоположной границы комнаты
  (set `self.SlowingFactor` SlowingFactor))

(event `self.ReceiveDestroyed`
  ;[0.2122 0.2122 0.2122] Движение и самоуничтожение при достижении противоположной границы комнаты
  (set `self.IsAlive` false))

(fn `SetupOakTrap`
  (bind (_returnvalue_x _returnvalue_y) (`KismetMathLibrary.BreakVector` (`self.K2_GetActorLocation` (`GameplayStatics.GetPlayerCharacter` 0))))
  ;[0.2122 0.2122 0.2122] Настройка размера и положения
  (`self.SetActorScale3D` (`KismetMathLibrary.MakeVector` (`KismetMathLibrary.RandomFloatInRange` 0.5 2.0) (`KismetMathLibrary.RandomFloatInRange` 0.5 2.0) (`KismetMathLibrary.RandomFloatInRange` 0.3 1.0)))
  (`self.K2_TeleportTo` (`KismetMathLibrary.MakeVector` 11300.0 _returnvalue_y (`KismetMathLibrary.RandomFloatInRange` 30.0 150.0)))
  ;[0.2122 0.2122 0.2122] Получение текущих параметров ловушки
  (bind _asddo_game_state (cast `/Game/GameplayFramework/DDO_GameState` (`GameplayStatics.GetGameState`)))
  (set `self.Damage` (`/Game/GameplayFramework/DDO_GameState.OakTrapDamage` _asddo_game_state))
  (set `self.Speed` (`/Game/GameplayFramework/DDO_GameState.OakTrapSpeed` _asddo_game_state)))

(fn `UserConstructionScript`)