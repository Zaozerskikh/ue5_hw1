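; FallingTrap_BP is a simple trap actor that damages the player when its Cube component hits them.
; On BeginPlay, SetupFallingTrap reads Damage from FallingTrapSettings_Table, picking the HardRoom or EasyRoom row by the DDO_GameState room difficulty flag.
; A hit on player character 0 passes the negated Damage and a trap type to ChangeHealth on DDO_PlayerState.
; The graphs contain no falling logic, only setup and hit handling.
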(event `self.Cube.OnComponentHit`
  (params (HitComponent :type "PrimitiveComponent Object Reference") (OtherActor :type "Actor Object Reference") (OtherComp :type "PrimitiveComponent Object Reference") (NormalImpulse :type "Vector Structure") (Hit :type "HitResult Structure (by ref)"))
  ;[0.2122 0.2122 0.2122] Столкновение с игроком
  (if (== (`GameplayStatics.GetPlayerCharacter` 0) OtherActor)
    (bind _asddo_player_state (cast `/Game/GameplayFramework/DDO_PlayerState` (`GameplayStatics.GetPlayerState` 0)))
    (`/Game/GameplayFramework/DDO_PlayerState.ChangeHealth` _asddo_player_state (* (`self.Damage`) -1.0) "NewEnumerator0")))

(event `self.ReceiveBeginPlay`
  (`self.SetupFallingTrap`))

(fn `SetupFallingTrap`
  ;[0.2122 0.2122 0.2122] Вычитывание настроек из таблицы
  (bind _asddo_game_state (cast `/Game/GameplayFramework/DDO_GameState` (`GameplayStatics.GetGameState`)))
  (if (`/Game/GameplayFramework/DDO_GameState.IsCurrentRoomHard` _asddo_game_state)
    (bind _returnvalue (`|GetDataTableRow` "/Game/Actors/Traps/SimpleTraps/FallingTrap/FallingTrapSettings_Table.FallingTrapSettings_Table" "HardRoom")
      (:`then`
        (set `self.Damage` (`.Damage_4_5A9CDF1A403608F2259318988342C22F` (break `/Game/Actors/Traps/SimpleTraps/FallingTrap/FallingTrapSettings_Struct` _returnvalue)))))
    (else
      (bind _returnvalue_2 (`|GetDataTableRow` "/Game/Actors/Traps/SimpleTraps/FallingTrap/FallingTrapSettings_Table.FallingTrapSettings_Table" "EasyRoom")
        (:`then`
          (set `self.Damage` (`.Damage_4_5A9CDF1A403608F2259318988342C22F` (break `/Game/Actors/Traps/SimpleTraps/FallingTrap/FallingTrapSettings_Struct` _returnvalue_2))))))))

(fn `UserConstructionScript`)