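; FallingTrapSpawner_BP periodically drops FallingTrap_BP traps in the player's path.
; On BeginPlay it reads the spawn interval from a settings DataTable, picking the hard or easy row by the GameState's IsCurrentRoomHard flag, and starts a looping timer.
; Each tick of that timer spawns a trap at a fixed height just ahead of the player along X, only while the player is within a set X range.
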(event `self.ReceiveBeginPlay`
  ;[0.2122 0.2122 0.2122] Вычитывание настроек из таблицы
  (bind _asddo_game_state (cast `/Game/GameplayFramework/DDO_GameState` (`GameplayStatics.GetGameState`)))
  (if (`/Game/GameplayFramework/DDO_GameState.IsCurrentRoomHard` _asddo_game_state)
    (bind _returnvalue (`|GetDataTableRow` "/Game/Actors/Traps/SimpleTraps/FallingTrap/FallingTrapSettings_Table.FallingTrapSettings_Table" "HardRoom")
      (:`then`
        (set `self.SpawnInterval` (break `/Game/Actors/Traps/SimpleTraps/FallingTrap/FallingTrapSettings_Struct` _returnvalue))))
    (else
      (bind _returnvalue_2 (`|GetDataTableRow` "/Game/Actors/Traps/SimpleTraps/FallingTrap/FallingTrapSettings_Table.FallingTrapSettings_Table" "EasyRoom")
        (:`then`
          (set `self.SpawnInterval` (break `/Game/Actors/Traps/SimpleTraps/FallingTrap/FallingTrapSettings_Struct` _returnvalue_2))))))
  ;[0.2122 0.2122 0.2122] Спавн ловушек
  (`KismetSystemLibrary.K2_SetTimerDelegate` (delegate `SpawnFallingTrap`) (`self.SpawnInterval`) true))

(event `SpawnFallingTrap`
  (bind (_returnvalue_x _returnvalue_y) (`KismetMathLibrary.BreakVector` (`self.K2_GetActorLocation` (`GameplayStatics.GetPlayerCharacter` 0))))
  (bind _returnvalue_x_2 (`KismetMathLibrary.BreakVector` (`self.K2_GetActorLocation` (`GameplayStatics.GetPlayerCharacter` 0))))
  ;[0.2122 0.2122 0.2122] Спавн ловушек
  (if (and (< _returnvalue_x_2 10500.0) (> _returnvalue_x_2 100.0))
    (`|SpawnActorFromClass` "/Game/Actors/Traps/SimpleTraps/FallingTrap/FallingTrap_BP.FallingTrap_BP_C" (`KismetMathLibrary.MakeTransform` (`KismetMathLibrary.MakeVector` (+ _returnvalue_x 500.0) _returnvalue_y 400.0)) "Undefined" "OverrideRootScale" null null)))

(fn `UserConstructionScript`)