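; Spawner actor that scatters damage zone traps across a room at BeginPlay.
; Its construction script reads the trap count from the settings data table, choosing the hard or easy room row from a game state flag.
; BeginPlay spawns traps at random positions snapped to a 100-unit grid within fixed bounds, skipping colliding spots and recounting all trap actors until the target is reached.
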(event `self.ReceiveBeginPlay`
  ;[0.2122 0.2122 0.2122] Спавн нужного количества ловушек
  (while (< (`self.CurrentDangerZoneCount`) (`self.TotalDangerZoneCount`))
    (`|SpawnActorFromClass` "/Game/Actors/Traps/SimpleTraps/DamageZoneTrap/DamageZoneTrap_BP.DamageZoneTrap_BP_C" (`KismetMathLibrary.Conv_VectorToTransform` (`KismetMathLibrary.MakeVector` (`KismetMathLibrary.Conv_IntToDouble` (* (/ (`KismetMathLibrary.Round` (`KismetMathLibrary.RandomFloatInRange` 500.0 10000.0)) 100) 100)) (`KismetMathLibrary.Conv_IntToDouble` (* (/ (`KismetMathLibrary.Round` (`KismetMathLibrary.RandomFloatInRange` 100.0 3400.0)) 100) 100)) 1.0)) "DontSpawnIfColliding" "OverrideRootScale" null null)
    (bind _outactors (`GameplayStatics.GetAllActorsOfClass` "/Game/Actors/Traps/SimpleTraps/DamageZoneTrap/DamageZoneTrap_BP.DamageZoneTrap_BP_C"))
    (set `self.CurrentDangerZoneCount` (`KismetArrayLibrary.Array_Length` _outactors))))

(fn `UserConstructionScript`
  ;[0.2122 0.2122 0.2122] Вычитывание количества ловушек в комнате из таблицы настроек
  (bind _asddo_game_state (cast `/Game/GameplayFramework/DDO_GameState` (`GameplayStatics.GetGameState`)))
  (if (`/Game/GameplayFramework/DDO_GameState.IsCurrentRoomHard` _asddo_game_state)
    (bind _returnvalue (`|GetDataTableRow` "/Game/Actors/Traps/SimpleTraps/DamageZoneTrap/DamageZoneSettings_Table.DamageZoneSettings_Table" "HardRoom")
      (:`then`
        (set `self.TotalDangerZoneCount` (break `/Game/Actors/Traps/SimpleTraps/DamageZoneTrap/DamgeZoneSettings_Struct` _returnvalue))))
    (else
      (bind _returnvalue_2 (`|GetDataTableRow` "/Game/Actors/Traps/SimpleTraps/DamageZoneTrap/DamageZoneSettings_Table.DamageZoneSettings_Table" "EasyRoom")
        (:`then`
          (set `self.TotalDangerZoneCount` (break `/Game/Actors/Traps/SimpleTraps/DamageZoneTrap/DamgeZoneSettings_Struct` _returnvalue_2)))))))