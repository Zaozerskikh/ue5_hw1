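; Damage zone trap that repeatedly drains the first player's health while an actor overlaps it.
; On BeginPlay it reads Damage from the shared FallingTrapSettings_Table, using the HardRoom or EasyRoom row according to the GameState's current-room flag.
; Overlap begin starts a fast looping DoDamage timer and overlap end pauses it, with no check on which actor overlaps.
; Each tick applies negative Damage through DDO_PlayerState's ChangeHealth with a trap type.
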(event `self.ReceiveActorEndOverlap`
  (params (OtherActor :type "Actor Object Reference"))
  ;[0.2122 0.2122 0.2122] Столкновения с игроком
  (`KismetSystemLibrary.K2_PauseTimer` null "DoDamage"))

(event `self.ReceiveActorBeginOverlap`
  (params (OtherActor :type "Actor Object Reference"))
  ;[0.2122 0.2122 0.2122] Столкновения с игроком
  (`KismetSystemLibrary.K2_SetTimer` null "DoDamage" 0.1 true))

(event `self.ReceiveBeginPlay`
  (`self.SetupDamageZoneTrap`))

(fn `DoDamage`
  ;[0.2122 0.2122 0.2122] Нанесение урона игроку
  (bind _asddo_player_state (cast `/Game/GameplayFramework/DDO_PlayerState` (`GameplayStatics.GetPlayerState` 0)))
  (`/Game/GameplayFramework/DDO_PlayerState.ChangeHealth` _asddo_player_state (* (`self.Damage`) -1.0) "NewEnumerator1"))

(fn `SetupDamageZoneTrap`
  ;[0.2122 0.2122 0.2122] Вычитывание настроек из таблицы
  (bind _asddo_game_state (cast `/Game/GameplayFramework/DDO_GameState` (`GameplayStatics.GetGameState`)))
  (if (`/Game/GameplayFramework/DDO_GameState.IsCurrentRoomHard` _asddo_game_state)
    (bind _returnvalue (`|GetDataTableRow` "/Game/Actors/Traps/SimpleTraps/FallingTrap/FallingTrapSettings_Table.FallingTrapSettings_Table" "HardRoom")
      (:`then`
        (set `self.Damage` (`.Damage_4_5A9CDF1A403608F2259318988342C22F` (break `/Game/Actors/Traps/SimpleTraps/FallingTrap/FallingTrapSettings_Struct` _returnvalue)))))
    (else
      (bind _returnvalue_2 (`|GetDataTableRow` "/Game/Actors/Traps/SimpleTraps/FallingTrap/FallingTrapSettings_Table.FallingTrapSettings_Table" "EasyRoom")
        (:`then`
          (set `self.Damage` (`.Damage_4_5A9CDF1A403608F2259318988342C22F` (break `/Game/Actors/Traps/SimpleTraps/FallingTrap/FallingTrapSettings_Struct` _returnvalue_2))))))))

(fn `UserConstructionScript`)